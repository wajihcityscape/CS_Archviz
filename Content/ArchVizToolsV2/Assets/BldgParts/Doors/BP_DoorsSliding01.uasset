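; Configurable ArchViz sliding door, static or movable, with an optional top window.
; The construction script sets meshes, width and opening offsets, materials and tint, then destroys unused components.
; A movable door with AutoOpen slides along local Y through a timeline on actor overlap, with open and close sounds.
; With multiple Materials, it binds to the player character's colour scheme event to swap door, frame and window materials at runtime.
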(event Custom|SwapDoorMaterial
  (params (SchemeID :type Integer))
  (bind _doorcolourtweak (Variables|MovableDoor|GetDoorColourTweak))
  (bind _materials (Variables|Materials|GetMaterials))
  (bind _output (Utilities|Array|Get(acopy) _materials SchemeID))
  ;[1 1 1] Swap colour
  (Rendering|Material|SetMaterial (select (Variables|MovableDoor|GetIsMovableDoor) (Variables|Default|GetDoorMovable) (Variables|Default|GetDoorStatic)) 0 (select (Variables|Materials|GetOneMaterialOnly) _output (Utilities|Array|Get(acopy) (Variables|Materials|GetMaterials_Door) SchemeID)))
  (if (Variables|MovableDoor|GetIsMovableDoor)
    (Rendering|Material|SetVectorParameterValueonMaterials (Variables|Default|GetDoorMovable) "Door-TintMovable" (Math|Conversions|ToVector(LinearColor) (Utilities|Array|Get(acopy) _doorcolourtweak (select (== (Utilities|Array|Length _doorcolourtweak) 1) 0 SchemeID)))))
  (Rendering|Material|SetMaterial (Variables|Default|GetFrame) 0 (select (Variables|Materials|GetOneMaterialOnly) _output (Utilities|Array|Get(acopy) (Variables|Materials|GetMaterials_Frame) SchemeID)))
  ;[1 1 1] Top Window
  (if (Variables|TopWindow|GetTopWindow)
    (Rendering|Material|SetMaterial (Variables|Default|GetFrameWindow) 0 (select (Variables|Materials|GetUseMaterials_Top) (Utilities|Array|Get(acopy) (Variables|Materials|GetMaterials_Top) SchemeID) _output))))

(event EventBeginPlay
  ;[1 1 1] Listen to colour scheme changes
  (bind _assdot_character_v2 (Utilities|Casting|CastToSDotCharacterV2 (Game|GetPlayerCharacter 0)))
  (if (> (Utilities|Array|Length (Variables|Materials|GetMaterials)) 1)
    (EventDispatchers|BindEventtoSwapColourScheme _assdot_character_v2 (delegate Custom|SwapDoorMaterial))))

(event Collision|EventActorBeginOverlap
  (params (OtherActor :type Actor%20Object%20Reference))
  (bind _defaultdoorlocation (Variables|MovableDoor|GetDefaultDoorLocation))
  ;[1 1 1] open close door
  (if (and (Variables|MovableDoor|GetAutoOpen) (Variables|MovableDoor|GetIsMovableDoor))
    (Audio|PlaySoundatLocation "/Game/ArchVizToolsV2/Sounds/Doors/S_DoorSlideA_Open.S_DoorSlideA_Open" "0, 0, 0" "0, 0, 0" 1.0 1.0 0.0 0 0 0)
    (bind _opendoor (Timeline|Timeline_0 Play)
      (:Update
        (if (Variables|MovableDoor|GetIsMovableDoor)
          (Transformation|SetRelativeLocation (Variables|Default|GetDoorMovable) (Math|Vector|MakeVector (.x _defaultdoorlocation) (+ (.y _defaultdoorlocation) (* (Variables|MovableDoor|GetDesiredOpening) _opendoor)) (.z _defaultdoorlocation)) false false))))))

(event Collision|EventActorEndOverlap
  (params (OtherActor :type Actor%20Object%20Reference))
  (bind _defaultdoorlocation (Variables|MovableDoor|GetDefaultDoorLocation))
  ;[1 1 1] open close door
  (if (and (Variables|MovableDoor|GetAutoOpen) (Variables|MovableDoor|GetIsMovableDoor))
    (Audio|PlaySoundatLocation "/Game/ArchVizToolsV2/Sounds/Doors/S_DoorSlideA_Close.S_DoorSlideA_Close" "0, 0, 0" "0, 0, 0" 1.0 1.0 0.0 0 0 0)
    (bind _opendoor (Timeline|Timeline_0 Reverse)
      (:Update
        (if (Variables|MovableDoor|GetIsMovableDoor)
          (Transformation|SetRelativeLocation (Variables|Default|GetDoorMovable) (Math|Vector|MakeVector (.x _defaultdoorlocation) (+ (.y _defaultdoorlocation) (* (Variables|MovableDoor|GetDesiredOpening) _opendoor)) (.z _defaultdoorlocation)) false false))))))

(fn ConstructionScript
  (bind _framewindow (Variables|Default|GetFrameWindow))
  (bind _framewindow_2 (Variables|Default|GetFrameWindow))
  (bind _materials (Variables|Materials|GetMaterials))
  (bind _defaultmaterial (Variables|Materials|GetDefaultMaterial))
  (bind _output (Utilities|Array|Get(acopy) _materials _defaultmaterial))
  (Utilities|FlowControl|Sequence
    (:then_0
      (Transformation|AddLocalOffset (Variables|Default|GetDoorMovable) (Math|Vector|MakeVector 0.0 (Utilities|Select :Index (Variables|DoorAndFrame|GetDoorWidth) :NewEnumerator0 -5.0 :NewEnumerator1 0.0 :NewEnumerator2 5.0) 0.0) false false)
      (Variables|MovableDoor|SetDefaultDoorLocation (Variables|/Script/Engine.SceneComponent|GetRelativeLocation (Variables|Default|GetDoorMovable)))
      (Transformation|AddLocalOffset (Variables|Default|GetDoorStatic) (Math|Vector|MakeVector 0.0 (* (Variables|DoorAndFrame|GetDoorOpening) -1.0) 0.0) false false)
      (if (Variables|TopWindow|GetTopWindow)
        (Transformation|SetRelativeScale3D _framewindow_2 (Variables|TopWindow|GetTopWindowScale))
        (Transformation|AddLocalOffset _framewindow_2 (Variables|TopWindow|GetTopWindowOffset) false false)))
    (:then_1
      (if (Variables|Materials|GetOneMaterialOnly)
        (Rendering|Material|SetMaterial (Variables|Default|GetFrame) 0 _output)
        (Rendering|Material|SetMaterial (Variables|Default|GetDoorMovable) 0 _output)
        (else
          (if (Variables|Materials|GetUseMaterials_Door)
            (Rendering|Material|SetMaterial (Variables|Default|GetDoorStatic) 0 (Utilities|Array|Get(acopy) (Variables|Materials|GetMaterials_Door) (Variables|Materials|GetDefaultMaterial))))
          (if (Variables|Materials|GetUseMaterials_Frame)
            (Rendering|Material|SetMaterial (Variables|Default|GetFrame) 0 (Utilities|Array|Get(acopy) (Variables|Materials|GetMaterials_Frame) (Variables|Materials|GetDefaultMaterial))))
          (if (Variables|Materials|GetUseMaterials_Top)
            (Rendering|Material|SetMaterial (Variables|Default|GetFrameWindow) 0 (Utilities|Array|Get(acopy) (Variables|Materials|GetMaterials_Top) (Variables|Materials|GetDefaultMaterial)))))))
    (:then_2
      (if (Variables|MovableDoor|GetIsMovableDoor)
        (Rendering|Material|SetVectorParameterValueonMaterials (Variables|Default|GetDoorMovable) "Door-TintMovable" (Math|Conversions|ToVector(LinearColor) (Utilities|Array|Get(acopy) (Variables|MovableDoor|GetDoorColourTweak) (Variables|MovableDoor|GetDoorColourTweakScenario))))))
    (:then_3
      (Components|StaticMesh|SetStaticMesh (Variables|Default|GetFrame) (Variables|DoorAndFrame|GetFrameMesh))
      (Components|StaticMesh|SetStaticMesh (select (Variables|MovableDoor|GetIsMovableDoor) (Variables|Default|GetDoorMovable) (Variables|Default|GetDoorStatic)) (Variables|DoorAndFrame|GetDoorMesh))
      (if (Variables|TopWindow|GetTopWindow)
        (Components|StaticMesh|SetStaticMesh _framewindow (Variables|TopWindow|GetTopMesh))
        (else
          (Components|DestroyComponent _framewindow)))
      (Components|DestroyComponent (select (Variables|MovableDoor|GetIsMovableDoor) (Variables|Default|GetDoorStatic) (Variables|Default|GetDoorMovable)))
      (if (Variables|MovableDoor|GetIsMovableDoor)
        (Transformation|SetRelativeTransform (Variables|Default|GetBox) (Variables|MovableDoor|GetCollisionBoxTransform) false false)
        (else
          (Components|DestroyComponent (Variables|Default|GetBox)))))))