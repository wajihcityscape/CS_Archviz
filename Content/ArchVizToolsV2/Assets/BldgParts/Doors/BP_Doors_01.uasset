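; Configurable archviz door actor with static or movable variants that can swing open automatically on overlap, with sound.
; The construction script picks meshes, offsets and scale from an AU, EU or US size preset or custom meshes, handles hinge side and top window, and destroys unused components.
; Materials follow a colour scheme ID, swapped at runtime through an SDotCharacterV2 event, with a tint parameter for movable doors.
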(event Custom|SwapDoorMaterial
  (params (SchemeID :type Integer))
  (bind _materials (Variables|Materials|GetMaterials))
  (bind _output (Utilities|Array|Get(acopy) _materials SchemeID))
  ;[1 1 1] Swap colour - Door and Handle
  (if (Variables|Materials|GetOneMaterialOnly)
    ;[1 1 1] One Material Only
    (Rendering|Material|SetMaterial (select (Variables|MovableDoor|GetIsMovableDoor) (Variables|Default|GetDoorMovable) (Variables|Default|GetDoorStatic)) 0 _output)
    (if (Variables|TopWindow|GetTopWindow)
      (Rendering|Material|SetMaterial (Variables|Default|GetFrameTop) 0 _output))
    (else
      (if (Variables|Materials|GetUseMaterials_Door)
        (CallFunction|SetMaterialsbyID (Variables|Materials|GetMaterials_Door) (select (Variables|MovableDoor|GetIsMovableDoor) (Variables|Default|GetDoorMovable) (Variables|Default|GetDoorStatic)) SchemeID))
      (if (Variables|Materials|GetUseMaterials_Handles)
        (CallFunction|SetMaterialsbyID (Variables|Materials|GetMaterials_Door) (select (Variables|MovableDoor|GetIsMovableDoor) (Variables|Default|GetHandleMovable) (Variables|Default|GetHandleStatic)) SchemeID))
      (if (Variables|MovableDoor|GetIsMovableDoor)
        (Rendering|Material|SetVectorParameterValueonMaterials (Variables|Default|GetDoorMovable) "Door-TintMovable" (Math|Conversions|ToVector(LinearColor) (Utilities|Array|Get(acopy) (Variables|MovableDoor|GetDoorColourTweak) SchemeID))))
      ;[1 1 1] Frame
      (if (Variables|Materials|GetUseMaterials_Frame)
        (CallFunction|SetMaterialsbyID (Variables|Materials|GetMaterials_Frame) (Variables|Default|GetDoorFrame) SchemeID))
      (if (Variables|TopWindow|GetTopWindow)
        (CallFunction|SetMaterialsbyID (Variables|Materials|GetMaterials_Top) (Variables|Default|GetFrameTop) SchemeID)))))

(event EventBeginPlay
  ;[1 1 1] Listen to colour scheme changes
  (bind _assdot_character_v2 (Utilities|Casting|CastToSDotCharacterV2 (Game|GetPlayerCharacter 0)))
  (if (> (Utilities|Array|Length (Variables|Materials|GetMaterials)) 1)
    (EventDispatchers|BindEventtoSwapColourScheme _assdot_character_v2 (delegate Custom|SwapDoorMaterial))))

(event Collision|EventActorBeginOverlap
  (params (OtherActor :type Actor%20Object%20Reference))
  (bind _doorinitialrotation (Variables|MovableDoor|GetDoorInitialRotation))
  (bind (_roll _pitch _yaw) (Math|Rotator|BreakRotator _doorinitialrotation))
  ;[1 1 1] open close door
  (if (Variables|MovableDoor|GetIsMovableDoor)
    (if (Variables|MovableDoor|GetAutoOpen)
      (bind _opendoor (Timeline|Timeline_0 Play)
        (:Update
          (if (Variables|MovableDoor|GetIsMovableDoor)
            (Transformation|SetWorldRotation (Variables|Default|GetDoorMovable) (Math|Rotator|MakeRotator _roll _pitch (+ (* (* (Variables|MovableDoor|GetDesiredRotation) (select (Variables|DoorSettings|GetHingeOnRight) 1.0 -1.0)) _opendoor) _yaw)) false false)))
        (:Opening%20sound
          (Utilities|FlowControl|FlipFlop
            (:A
              (Audio|PlaySoundatLocation "/Game/ArchVizToolsV2/Sounds/Doors/S_DoorA_Open.S_DoorA_Open" "0, 0, 0" "0, 0, 0" 1.0 1.0 0.0 0 0 0))
            (:B
              (Audio|PlaySoundatLocation "/Game/ArchVizToolsV2/Sounds/Doors/S_DoorA_Close.S_DoorA_Close" "0, 0, 0" "0, 0, 0" 1.0 1.0 0.0 0 0 0))))))))

(event Collision|EventActorEndOverlap
  (params (OtherActor :type Actor%20Object%20Reference))
  (bind _doorinitialrotation (Variables|MovableDoor|GetDoorInitialRotation))
  (bind (_roll _pitch _yaw) (Math|Rotator|BreakRotator _doorinitialrotation))
  ;[1 1 1] open close door
  (if (Variables|MovableDoor|GetIsMovableDoor)
    (if (Variables|MovableDoor|GetAutoOpen)
      (bind _opendoor (Timeline|Timeline_0 Reverse)
        (:Update
          (if (Variables|MovableDoor|GetIsMovableDoor)
            (Transformation|SetWorldRotation (Variables|Default|GetDoorMovable) (Math|Rotator|MakeRotator _roll _pitch (+ (* (* (Variables|MovableDoor|GetDesiredRotation) (select (Variables|DoorSettings|GetHingeOnRight) 1.0 -1.0)) _opendoor) _yaw)) false false)))
        (:Opening%20sound
          (Utilities|FlowControl|FlipFlop
            (:A
              (Audio|PlaySoundatLocation "/Game/ArchVizToolsV2/Sounds/Doors/S_DoorA_Open.S_DoorA_Open" "0, 0, 0" "0, 0, 0" 1.0 1.0 0.0 0 0 0))
            (:B
              (Audio|PlaySoundatLocation "/Game/ArchVizToolsV2/Sounds/Doors/S_DoorA_Close.S_DoorA_Close" "0, 0, 0" "0, 0, 0" 1.0 1.0 0.0 0 0 0))))))))

(fn ConstructionScript
  (bind _doorvalues (CallFunction|GetDoorID))
  (bind _materials (Variables|Materials|GetMaterials))
  (bind _frametop (Variables|Default|GetFrameTop))
  (bind _doorrelativelocation (Variables|Default|GetDoorRelativeLocation))
  (bind _frametop_2 (Variables|Default|GetFrameTop))
  (bind _doorrelativelocation_2 (Variables|Default|GetDoorRelativeLocation))
  (bind _defaultcolourscheme (Variables|Materials|GetDefaultColourScheme))
  (bind _topwindowoffset (Variables|TopWindow|GetTopWindowOffset))
  (bind (_doorsizeid _frame _door _frametop_3 _dooroffset _handleoffset _topheightoffset _scalewidth _scaleheight) (Utilities|Struct|BreakBPS_DoorSizes _doorvalues))
  (bind (_x _y _z) (Math|Vector|BreakVector _topwindowoffset))
  (bind _output (Utilities|Array|Get(acopy) _materials _defaultcolourscheme))
  (Utilities|FlowControl|Sequence
    (:then_0
      ;[1 1 1] set materials
      (if (Variables|Materials|GetOneMaterialOnly)
        (Rendering|Material|SetMaterial (Variables|Default|GetDoorFrame) 0 _output)
        (Rendering|Material|SetMaterial (Variables|Default|GetDoorMovable) 0 _output)
        (else
          (if (Variables|Materials|GetUseMaterials_Door)
            (CallFunction|SetMaterialsbyID (Variables|Materials|GetMaterials_Door) (select (Variables|MovableDoor|GetIsMovableDoor) (Variables|Default|GetDoorMovable) (Variables|Default|GetDoorStatic)) (Variables|Materials|GetDefaultColourScheme)))
          (if (Variables|Materials|GetUseMaterials_Frame)
            (CallFunction|SetMaterialsbyID (Variables|Materials|GetMaterials_Frame) (Variables|Default|GetDoorFrame) (Variables|Materials|GetDefaultColourScheme)))
          (if (Variables|Materials|GetUseMaterials_Top)
            (CallFunction|SetMaterialsbyID (Variables|Materials|GetMaterials_Top) (Variables|Default|GetFrameTop) (Variables|Materials|GetDefaultColourScheme)))
          (if (Variables|Materials|GetUseMaterials_Handles)
            (CallFunction|SetMaterialsbyID (Variables|Materials|GetMaterials_Handles) (select (Variables|MovableDoor|GetIsMovableDoor) (Variables|Default|GetHandleMovable) (Variables|Default|GetHandleStatic)) (Variables|Materials|GetDefaultColourScheme))))))
    (:then_1
      ;[1 1 1] set frame
      (Components|StaticMesh|SetStaticMesh (Variables|Default|GetDoorFrame) (select (Variables|Meshes|GetUseCustomFrame) (Variables|Meshes|GetFrameMesh) (.Frame (Utilities|Struct|BreakBPS_DoorSizes (.DoorValues (CallFunction|GetDoorID))))))
      ;[1 1 1] set door
      (Components|StaticMesh|SetStaticMesh (select (Variables|MovableDoor|GetIsMovableDoor) (Variables|Default|GetDoorMovable) (Variables|Default|GetDoorStatic)) (select (Variables|Meshes|GetUseCustomDoor) (Variables|Meshes|GetDoorMesh) (.Door (Utilities|Struct|BreakBPS_DoorSizes (.DoorValues (CallFunction|GetDoorID))))))
      ;[1 1 1] set handle
      (Components|StaticMesh|SetStaticMesh (select (Variables|MovableDoor|GetIsMovableDoor) (Variables|Default|GetHandleMovable) (Variables|Default|GetHandleStatic)) (Variables|Meshes|GetHandleMesh)))
    (:then_2
      ;[1 1 1] offset scale rotation
      (Transformation|AddLocalOffset (Variables|Default|GetDoorMovable) (Math|Vector|MakeVector (.x _doorrelativelocation_2) (.DoorOffset (Utilities|Struct|BreakBPS_DoorSizes (.DoorValues (CallFunction|GetDoorID)))) (.z _doorrelativelocation_2)) false false)
      (Transformation|AddLocalOffset (Variables|Default|GetHandleStatic) (Math|Vector|MakeVector (.x _doorrelativelocation) (.HandleOffset (Utilities|Struct|BreakBPS_DoorSizes (.DoorValues (CallFunction|GetDoorID)))) (.z _doorrelativelocation)) false false)
      (Transformation|SetRelativeRotation (Variables|Default|GetDoorStatic) (Math|Rotator|MakeRotator 0.0 0.0 (* (Variables|DoorSettings|GetDoorRotation) -1.0)) false false)
      (if (Variables|DoorSettings|GetHingeOnRight)
        _
        (else
          (Transformation|SetRelativeScale3D (Variables|Default|GetDoorFrame) "1.000000,-1.000000,1.000000")))
      ;[1 1 1] top window
      (if (Variables|TopWindow|GetTopWindow)
        (Transformation|SetRelativeScale3D _frametop_2 (Variables|TopWindow|GetTopWindowScale))
        (Transformation|AddLocalOffset _frametop_2 (Math|Vector|MakeVector _x _y (+ _z (.TopHeightOffset (Utilities|Struct|BreakBPS_DoorSizes (.DoorValues (CallFunction|GetDoorID)))))) false false))
      ;[1 1 1] Overall Scale (international format)
      (Transformation|SetRelativeScale3D (Variables|Default|GetDoorFrame) (Math|Vector|MakeVector 1.0 (select (Variables|DoorSettings|GetHingeOnRight) _scalewidth (* _scalewidth -1.0)) _scaleheight)))
    (:then_3
      ;[1 1 1] movable door colour tweak
      (if (Variables|MovableDoor|GetIsMovableDoor)
        (Rendering|Material|SetVectorParameterValueonMaterials (Variables|Default|GetDoorMovable) "Door-TintMovable" (Math|Conversions|ToVector(LinearColor) (Utilities|Array|Get(acopy) (Variables|MovableDoor|GetDoorColourTweak) (Variables|MovableDoor|GetDoorColourTweakScenario))))
        (Variables|MovableDoor|SetDoorInitialRotation (Transformation|GetWorldRotation (Variables|Default|GetDoorMovable)))
        (Transformation|SetRelativeScale3D (Variables|Default|GetBox) (Variables|MovableDoor|GetCollisionScale))
        (Transformation|AddRelativeLocation (Variables|Default|GetBox) (Variables|MovableDoor|GetCollisionLocationOffset) false false)))
    (:then_4
      ;[1 1 1] remove obsolete meshes
      (if (Variables|TopWindow|GetTopWindow)
        (Components|StaticMesh|SetStaticMesh _frametop (Variables|TopWindow|GetTopMesh))
        (else
          (Components|DestroyComponent _frametop)))
      (Components|DestroyComponent (select (Variables|MovableDoor|GetIsMovableDoor) (Variables|Default|GetDoorStatic) (Variables|Default|GetDoorMovable)))
      (Components|DestroyComponent (select (Variables|MovableDoor|GetIsMovableDoor) (Variables|Default|GetHandleStatic) (Variables|Default|GetHandleMovable)))
      (if (not (Variables|MovableDoor|GetIsMovableDoor))
        (Components|DestroyComponent (Variables|Default|GetBox))))))

(fn SetMaterialsbyID
  (params (Materials :type Array%20of%20BPS%20Mat%20with%20ID%20Structures) (Mesh :type Static%20Mesh%20Component%20Object%20Reference) (ColourSchemeID :type Integer))
  (for _array_element Materials
    (if (== (.ColorSchemeID (Utilities|Struct|BreakBPS_MatWithID _array_element)) ColourSchemeID)
      (Rendering|Material|SetMaterial Mesh (.MatID (Utilities|Struct|BreakBPS_MatWithID _array_element)) (.Material (Utilities|Struct|BreakBPS_MatWithID _array_element))))))

(fn GetDoorID
  (bind _doorsizes (Variables|DoorSettings|GetDoorSizes))
  (bind _returnvalue (Utilities|Select :Index _doorsizes :NewEnumerator12 0 :NewEnumerator2 1 :NewEnumerator9 2 :NewEnumerator13 3 :NewEnumerator15 4 :NewEnumerator14 5 :NewEnumerator0 6 :NewEnumerator16 7 :NewEnumerator17 8 :NewEnumerator18 9 :NewEnumerator19 10 :NewEnumerator20 11 :NewEnumerator1 12 :NewEnumerator6 13 :NewEnumerator7 14 :NewEnumerator11 15 :NewEnumerator8 16 :NewEnumerator10 17 :NewEnumerator21 18 :NewEnumerator22 19 :NewEnumerator23 20))
  (return (Utilities|Array|Get(acopy) (Variables|Default|GetDoorSizesStructure) _returnvalue) _returnvalue))