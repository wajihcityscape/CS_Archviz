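; BP_SwapFan01 is an arch-viz fan appliance with constantly spinning blades and a swappable blade material.
; On BeginPlay it binds to the SDotCharacterV2 player's swap-by-code event and responds when the item tag matches its own.
; The variation ID selects a blade material from an array; despite the mesh-swap naming, only the material changes.
; The construction script applies the default choice, and Tick adds yaw without delta-time scaling.
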(event Custom|UseSelectedMesh
  (params (ChoiceID :type Integer))
  ;[1 1 1] Swap materials
  (bind _output_get (Variables|CeilingFan|SetDefaultMeshID ChoiceID))
  (Rendering|Material|SetMaterial (Variables|Default|GetP_HunterCFan01_blades) 0 (Utilities|Array|Get(acopy) (Variables|CeilingFan|GetMaterials) _output_get)))

(event Custom|SwapBlades
  (params (ItemTag :type String) (VariationID :type Integer))
  ;[1 1 1] Listen to changes
  (if (Utilities|Enum|Equal(Enum) ItemTag (Variables|CeilingFan|GetItemTagIn))
    (CallFunction|UseSelectedMesh VariationID)
    (Development|PrintString (Utilities|String|Append "Tag recieved:  " ""))))

(event EventBeginPlay
  ;[1 1 1] Listen to changes
  (bind _assdot_character_v2 (Utilities|Casting|CastToSDotCharacterV2 (Game|GetPlayerCharacter 0)))
  (EventDispatchers|BindEventtoSwapMeshbyCode _assdot_character_v2 (delegate Custom|SwapBlades)))

(event EventTick
  (params (DeltaSeconds :type Float%20%28single-precision%29))
  ;[1 1 1] Rotate blades
  (Transformation|AddRelativeRotation (Variables|Default|GetP_HunterCFan01_blades) (Math|Rotator|MakeRotator 0.0 0.0 (Variables|CeilingFan|GetBladeRotation)) false false))

(fn ConstructionScript
  (CallFunction|UseSelectedMesh (Variables|CeilingFan|GetDefaultMeshID)))