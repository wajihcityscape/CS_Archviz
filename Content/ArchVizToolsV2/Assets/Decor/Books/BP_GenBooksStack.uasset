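; Decor actor that procedurally builds a row of varied books along local Y as instanced static meshes in the Construction Script.
; A seeded random stream picks each book's width, height and length within set ranges, with GenerateBooks acting as a one-shot reseed toggle.
; Cumulative widths set positions, and sizes become scales relative to mesh bounds.
; Index 0 only seeds the offsets, and RandomAngels reuses book width as pitch.
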(event EventBeginPlay)

(event Collision|EventActorBeginOverlap
  (params (OtherActor :type Actor%20Object%20Reference)))

(event EventTick
  (params (DeltaSeconds :type Float%20%28single-precision%29)))

(fn ConstructionScript
  (bind _instancedstaticmesh (Variables|Default|GetInstancedStaticMesh))
  (bind (_min _max) (Components|StaticMesh|GetLocalBounds _instancedstaticmesh))
  (bind _returnvalue (- _min _max))
  (bind _returnvalue_2 (Math|Float|Absolute(Float) (.y _returnvalue)))
  (bind _returnvalue_3 (Math|Float|Absolute(Float) (.z _returnvalue)))
  (bind _returnvalue_4 (Math|Float|Absolute(Float) (.x _returnvalue)))
  ;[1 1 1] Random Stream
  (if (Variables|Random|GetGenerateBooks)
    (Class|KismetMathLibrary|SeedRandomStream (Variables|Random|GetRandomStream)))
  (Variables|Random|SetGenerateBooks false)
  ;[1 1 1] replace materials and meshes
  (Components|StaticMesh|SetStaticMesh (Variables|Default|GetInstancedStaticMesh) (Variables|Book|GetBook%20Mesh))
  (Rendering|Material|SetMaterial (Variables|Default|GetInstancedStaticMesh) 0 (Variables|Book|GetBookMaterial))
  ;[1 1 1] create random values
  (for _index (range 0 (- (Variables|BookStack|GetNumberOfBooks) 1))
    (if (== _index 0)
      (Utilities|Array|Add (Variables|BookStack|GetInstancedBookWidth) _returnvalue_2)
      (Utilities|Array|Add (Variables|BookStack|GetInstancedBookHeight) _returnvalue_3)
      (Utilities|Array|Add (Variables|BookStack|GetInstancedBookLength) _returnvalue_4)
      (Utilities|Array|Add (Variables|BookStack|GetStackTransformY) 0.0)
      (else
        (Utilities|Array|Add (Variables|BookStack|GetInstancedBookWidth) (Math|Float|Lerp (Variables|BookStack|GetBookMaxWidth) (Variables|BookStack|GetBookMinWidth) (Math|Random|RandomFloatfromStream (Variables|Random|GetRandomStream))))
        (Utilities|Array|Add (Variables|BookStack|GetInstancedBookHeight) (Math|Float|Lerp (Variables|BookStack|GetBookMaxHeight) (Variables|BookStack|GetBookMinHeight) (Math|Random|RandomFloatfromStream (Variables|Random|GetRandomStream))))
        (Utilities|Array|Add (Variables|BookStack|GetInstancedBookLength) (Math|Float|Lerp (Variables|BookStack|GetBookMaxLength) (Variables|BookStack|GetBookMinLength) (Math|Random|RandomFloatfromStream (Variables|Random|GetRandomStream))))
        (Utilities|Array|Add (Variables|BookStack|GetStackTransformY) (+ (Utilities|Array|Get(acopy) (Variables|BookStack|GetStackTransformY) (- _index 1)) (Utilities|Array|Get(acopy) (Variables|BookStack|GetInstancedBookWidth) (- _index 1)))))))
  ;[1 1 1] create book instances
  (for (_array_element _array_index) (Variables|BookStack|GetStackTransformY)
    (if (not (== _array_index 0))
      (Components|InstancedStaticMesh|AddInstance (Variables|Default|GetInstancedStaticMesh) (Math|Transform|MakeTransform (Math|Vector|MakeVector 0.0 _array_element 0.0) (Math|Rotator|MakeRotator 0.0 (select (Variables|Random|GetRandomAngels) (Utilities|Array|Get(acopy) (Variables|BookStack|GetInstancedBookWidth) _array_index) 0.0) 0.0) (Math|Vector|MakeVector (/ (Utilities|Array|Get(acopy) (Variables|BookStack|GetInstancedBookLength) _array_index) _returnvalue_4) (/ (Utilities|Array|Get(acopy) (Variables|BookStack|GetInstancedBookWidth) _array_index) _returnvalue_2) (/ (Utilities|Array|Get(acopy) (Variables|BookStack|GetInstancedBookHeight) _array_index) _returnvalue_3)))))))